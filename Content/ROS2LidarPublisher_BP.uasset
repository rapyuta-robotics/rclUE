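; ROS2LidarPublisher_BP is a ROS 2 publisher that sends lidar data as laser scan messages.
; On UpdateandPublishMessage it casts the topic message to a laser scan message, fills it with the Lidar's ROS 2 data and publishes it.
; BeginPlay and EndPlay only forward to the parent class, and Tick is disabled.
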(event `self.ReceiveBeginPlay`
  (`parent.ReceiveBeginPlay`))

(event `self.ReceiveEndPlay`
  (params (EndPlayReason :type "EEndPlayReason Enum" :default "Destroyed"))
  (`parent.ReceiveEndPlay` EndPlayReason))

(event `self.UpdateAndPublishMessage`
  (bind _asros2laser_scan_msg (cast `ROS2LaserScanMsg` (`ROS2Topic.Msg` (`self.Topic`))))
  (`ROS2LaserScanMsg.Update` _asros2laser_scan_msg (`SensorLidar.GetROS2Data` (`self.Lidar`)))
  (`self.Publish`))