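; BP_TestServiceClient is a test ROS 2 service client that sends an addition request and displays the answer.
; On BeginPlay it binds request and answer delegates on its ROS2ServiceClient.
; The request handler fills a ROS2TestSrv with two random integers.
; The answer handler reads the inputs and output back and writes them as a sum equation to a widget's response text, if that widget is valid.
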(event `SetRequestData`
  (params (Service :type "ROS2GenericSrv Object Reference"))
  (bind _asros2test_srv (cast `ROS2TestSrv` Service))
  (`ROS2TestSrv.SetInputs` _asros2test_srv (`KismetMathLibrary.RandomInteger64InRange` 0 1000) (`KismetMathLibrary.RandomInteger64InRange` 0 1000)))

(event `self.ReceiveBeginPlay`
  (bind _ros2serviceclient (`self.ROS2ServiceClient`))
  (set `ROS2ServiceClient.RequestDelegate` (delegate `SetRequestData`) _ros2serviceclient)
  (set `ROS2ServiceClient.AnswerDelegate` (delegate `GetResponseData`) _ros2serviceclient))

(event `GetResponseData`
  (params (Service :type "ROS2GenericSrv Object Reference"))
  (bind _asros2test_srv (cast `ROS2TestSrv` Service :!pure true))
  (bind _widget (`self.Widget`))
  (`/Engine/EditorBlueprintResources/StandardMacros.IsValid` _widget
    (:`Is Valid`
      (bind _res (`ROS2TestSrv.GetOutput` _asros2test_srv))
      (bind (_a _b) (`ROS2TestSrv.GetInputs` _asros2test_srv))
      (set `/rclUE/Widgets/ROS2_Widget_Main.ServiceResponseText` (`KismetTextLibrary.Conv_StringToText` (`KismetStringLibrary.Concat_StrStr` (`KismetStringLibrary.Conv_IntToString` (`KismetMathLibrary.Conv_Int64ToInt` _a)) " + " (`KismetStringLibrary.Conv_IntToString` (`KismetMathLibrary.Conv_Int64ToInt` _b)) " = " (`KismetStringLibrary.Conv_IntToString` (`KismetMathLibrary.Conv_Int64ToInt` _res)))) _widget))))

(fn `UserConstructionScript`)