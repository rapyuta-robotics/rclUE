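; A ROS 2 string publisher Blueprint that supplies "HelloWorld" messages with an incrementing counter.
; On BeginPlay it assigns an event to UpdateDelegate.
; PublishString casts the given topic message to ROS2StringMsg, updates it with "HelloWorld" plus the current NCall value, then increments NCall.
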(event `self.ReceiveBeginPlay`
  (set `self.UpdateDelegate` (`|CreateDelegate` :!event `PublishString`)))

(fn `PublishString`
  (params (TopicMessage :type "ROS2GenericMsg Object Reference"))
  (bind _ncall (`self.NCall`))
  (`ROS2StringMsg.Update` (cast `ROS2StringMsg` TopicMessage :!pure true) (`KismetStringLibrary.Concat_StrStr` "HelloWorld" (`KismetStringLibrary.Conv_IntToString` _ncall)))
  (set `self.NCall` (+ _ncall 1))
  (return))