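; Test actor for a ROS 2 Fibonacci action server, apparently incomplete or with broken wiring.
; Goal acceptance resets the sequence and sends a response; cancellation sends its response and clears the timer.
; Feedback and result handlers only cast the action, and CalculateFibonacci only casts and stores it without starting a timer.
; GetNextFibonacci is empty, with its sequence-step and feedback/result logic left disconnected.
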(event `self.ReceiveBeginPlay`)

(event `SetFeedback`
  (params (Action :type "ROS2GenericAction Object Reference"))
  (cast `ROS2FibonacciAction` Action))

(event `SetResult`
  (params (Action :type "ROS2GenericAction Object Reference"))
  (cast `ROS2FibonacciAction` Action))

(event `CalculateFibonacci`
  (params (Action :type "ROS2GenericAction Object Reference"))
  (bind _asros2fibonacci_action (cast `ROS2FibonacciAction` Action))
  (set `self.As ROS2Fibonacci Action` _asros2fibonacci_action))

(event `Cancel Goal`
  (`ROS2ActionServer.ProcessAndSendCancelResponse` (`self.ROS2ActionServer`))
  (`KismetSystemLibrary.K2_ClearAndInvalidateTimerHandle` (`self.FibonacciTimerHandle`)))

(event `Accept Goal`
  (set `self.FibonacciSequence` (`self.FibonacciInit`))
  (`ROS2ActionServer.SendGoalResponse` (`self.ROS2ActionServer`)))

(fn `GetNextFibonacci`)

(fn `UserConstructionScript`)