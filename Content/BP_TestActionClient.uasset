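; BP_TestActionClient is a test client for a ROS 2 Fibonacci action, with a widget for status.
; Requesting results calls the action client and sets the widget's cancel action flag, which cancel confirmation clears.
; Goal, feedback and result events only cast the action.
; SetWidgetText concatenates array elements and colors partial and final text differently, but its event graph calls are disconnected, so no sequence is displayed.
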(event `self.ReceiveBeginPlay`)

(event `SetGoalInput`
  (params (Action :type "ROS2GenericAction Object Reference"))
  (cast `ROS2FibonacciAction` Action))

(event `UpdateWithFeedback`
  (params (Action :type "ROS2GenericAction Object Reference"))
  (cast `ROS2FibonacciAction` Action))

(event `UpdateWithResult`
  (params (Action :type "ROS2GenericAction Object Reference"))
  (cast `ROS2FibonacciAction` Action))

(event `Request Results`
  (`ROS2ActionClient.GetResultRequest` (`self.ROS2ActionClient`))
  (`/rclUE/Widgets/WBP_ROS2_Widget_Main.SetCancelAction` (`self.Widget`) true))

(event `Cancel Confirmed`
  (`/rclUE/Widgets/WBP_ROS2_Widget_Main.SetCancelAction` (`self.Widget`) false))

(fn `SetWidgetText`
  (params (Array :type "Array of Integer") (Partial :type Boolean))
  (locals (Result :type String))
  (bind _widget (`self.Widget`))
  (for _array_element Array
    (set `local.Result` (`KismetStringLibrary.Concat_StrStr` (`local.Result`) (`KismetStringLibrary.Conv_IntToString` _array_element) " ")))
  (`/Engine/EditorBlueprintResources/StandardMacros.IsValid` _widget
    (:`Is Valid`
      (set `/rclUE/Widgets/WBP_ROS2_Widget_Main.ActionResponseText` (`KismetTextLibrary.Conv_StringToText` (`local.Result`)) _widget)
      (if Partial
        (set `/rclUE/Widgets/WBP_ROS2_Widget_Main.TextColor` (struct :`R` 0.276042 :`G` 0.010469 :`A` 1.0) _widget)
        (else
          (set `/rclUE/Widgets/WBP_ROS2_Widget_Main.TextColor` (struct :`G` 0.192708 :`B` 0.014257 :`A` 1.0) _widget)))
      (return))))

(fn `UserConstructionScript`)